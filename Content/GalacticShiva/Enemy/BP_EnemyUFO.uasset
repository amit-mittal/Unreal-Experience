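; BP_EnemyUFO is an enemy UFO that flies in a straight line toward where the player was when it spawned.
; BeginPlay reads the player character's location and rotates the UFO to face it once, with no later homing.
; Tick adds Velocity along that stored forward direction and sets the location without sweep.
; The step is not scaled by delta time, so speed depends on frame rate.
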(event EventBeginPlay
  (bind _asbp_player_character (Utilities|Casting|CastToBP_PlayerCharacter (Game|GetPlayerCharacter 0)))
  (Variables|Default|SetPlayerLocation (Transformation|GetActorLocation _asbp_player_character))
  (Variables|Default|SetEnemyCharacter (Transformation|GetActorLocation))
  (bind _output_get (Variables|Default|SetRotation (Math|Rotator|FindLookatRotation (Variables|Default|GetEnemyCharacter) (Variables|Default|GetPlayerLocation))))
  (Transformation|SetActorRotation _output_get))

(event Collision|EventActorBeginOverlap
  (params (OtherActor :type Actor%20Object%20Reference)))

(event EventTick
  (params (DeltaSeconds :type Float%20%28single-precision%29))
  (bind _output_get (Variables|Default|SetEnemyCharacter (+ (Variables|Default|GetEnemyCharacter) (* (Variables|Default|GetVelocity) (Math|Vector|GetForwardVector (Variables|Default|GetRotation))))))
  (Transformation|SetActorLocation _output_get false false))

(fn ConstructionScript)